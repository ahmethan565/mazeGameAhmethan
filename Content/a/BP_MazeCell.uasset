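; BP_MazeCell is a modular maze tile that builds its own walls, ceiling and light.
; The construction script scales the floor to GridSize and adds scaled meshes for each enabled wall and ceiling, with thickness proportional to cell size.
; A positive LightIntensity adds a centered point light near the top.
; At BeginPlay it binds to the player character's maze gate event, recoloring that light to the character's LightColor when Isınside is false.
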(event Custom|MazeGate_Event
  (params (Isınside? :type Boolean))
  (bind _pointlight (Variables|Default|GetpointLight))
  (if (not Isınside?)
    (Utilities|IsValid _pointlight
      (:Is%20Valid
        (Rendering|Components|Light|SetLightColor _pointlight (Variables|/Game/ThirdPerson/Blueprints/BP_ThirdPersonCharacter.BP_ThirdPersonCharacter_C|GetlightColor (Variables|Default|GetThird%20Person%20Char)) true)))))

(event EventBeginPlay
  (bind _asbp_third_person_character (Utilities|Casting|CastToBP_ThirdPersonCharacter (Game|Player|GetPlayerPawn 0)))
  (Variables|Default|SetThird%20Person%20Char _asbp_third_person_character)
  (EventDispatchers|BindEventtoMazeGate _asbp_third_person_character (delegate Custom|MazeGate_Event)))

(event Collision|EventActorBeginOverlap
  (params (OtherActor :type Actor%20Object%20Reference)))

(event EventTick
  (params (DeltaSeconds :type Float%20%28single-precision%29)))

(fn ConstructionScript
  (bind _gridsize (Variables|Default|GetgridSize))
  (LocalVariables|SetwallLenght _gridsize)
  (LocalVariables|SetWallTickness (* _gridsize 0.1))
  (Transformation|SetRelativeScale3D (Variables|Default|Getfloor) (Utilities|SizetoCubeScale (Math|Vector|MakeVector (LocalVariables|GetwallLenght) (LocalVariables|GetwallLenght) (LocalVariables|GetWallTickness))))
  (if (Variables|Default|Getwest)
    (AddComponent|AddStaticMeshComponent false (Math|Transform|MakeTransform (Math|Vector|MakeVector 0.0 0.0 0.0) "0, 0, 0" (Utilities|SizetoCubeScale (Math|Vector|MakeVector (LocalVariables|GetwallLenght) (LocalVariables|GetWallTickness) (Variables|Default|GetWallHeight))))))
  (if (Variables|Default|Geteast)
    (AddComponent|AddStaticMeshComponent false (Math|Transform|MakeTransform (Math|Vector|MakeVector 0.0 (- (LocalVariables|GetwallLenght) (LocalVariables|GetWallTickness)) 0.0) "0, 0, 0" (Utilities|SizetoCubeScale (Math|Vector|MakeVector (LocalVariables|GetwallLenght) (LocalVariables|GetWallTickness) (Variables|Default|GetWallHeight))))))
  (if (Variables|Default|Getsouth)
    (AddComponent|AddStaticMeshComponent false (Math|Transform|MakeTransform (Math|Vector|MakeVector 0.0 0.0 0.0) "0, 0, 0" (Utilities|SizetoCubeScale (Math|Vector|MakeVector (LocalVariables|GetWallTickness) (LocalVariables|GetwallLenght) (Variables|Default|GetWallHeight))))))
  (if (Variables|Default|Getnorth)
    (AddComponent|AddStaticMeshComponent false (Math|Transform|MakeTransform (Math|Vector|MakeVector (- (LocalVariables|GetwallLenght) (LocalVariables|GetWallTickness)) 0.0 0.0) "0, 0, 0" (Utilities|SizetoCubeScale (Math|Vector|MakeVector (LocalVariables|GetWallTickness) (LocalVariables|GetwallLenght) (Variables|Default|GetWallHeight))))))
  (if (Variables|Default|Getcelling)
    (AddComponent|AddStaticMeshComponent false (Math|Transform|MakeTransform (Math|Vector|MakeVector 0.0 0.0 (Variables|Default|GetWallHeight)) "0, 0, 0" (Utilities|SizetoCubeScale (Math|Vector|MakeVector (LocalVariables|GetwallLenght) (LocalVariables|GetwallLenght) (LocalVariables|GetWallTickness))))))
  (if (> (Variables|Default|GetlightIntensity) 0.0)
    (bind _returnvalue (AddComponent|AddPointLightComponent false (Math|Transform|MakeTransform (Math|Vector|MakeVector (* (LocalVariables|GetwallLenght) 0.5) (* (LocalVariables|GetwallLenght) 0.5) (* (Variables|Default|GetWallHeight) 0.9)) "0, 0, 0" "1.000000,1.000000,1.000000")))
    (bind _output_get (Variables|Default|SetpointLight _returnvalue))
    (Rendering|Components|Light|SetIntensity _output_get (Variables|Default|GetlightIntensity))
    (Rendering|Components|Light|SetLightColor _output_get (Variables|Default|GetlightColor) true)))