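; BP_Door is an interactable locked door that slides open when the game mode's Keys value equals the door's KeyNumber.
; On BeginPlay it caches gameMode1, and Interact either plays the Door_Rotate timeline or prints a wrong-key message.
; Despite its name, the timeline moves the Cube's relative location between StartLocation and FinishLocation rather than rotating it.
; The construction script applies the Material variable to the Cube.
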(event EventInteract
  (if (== (Variables|/Game/a/gameMode1.gameMode1_C|GetKeys (Variables|Default|GetgameMode)) (Variables|Default|GetKeyNumber))
    (bind _newtrack_0 (Timeline|Door_Rotate Play)
      (:Update
        (Transformation|SetRelativeLocation (Variables|Default|GetCube) (Math|Vector|Lerp(Vector) (Variables|Default|GetstartLocation) (Variables|Default|GetfinishLocation) _newtrack_0) false false)))
    (else
      (Development|PrintString "wrong key"))))

(event EventBeginPlay
  (bind _asgame_mode_1 (Utilities|Casting|CastTogameMode1 (Game|GetGameMode)))
  (Variables|Default|SetgameMode _asgame_mode_1))

(fn ConstructionScript
  (Rendering|Material|SetMaterial (Variables|Default|GetCube) 0 (Variables|Default|Getmaterial)))