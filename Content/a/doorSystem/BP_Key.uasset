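; BP_Key is a key pickup for the door system, recording its key number in the game mode when interacted with.
; BeginPlay caches the gameMode1 reference, and Interact overwrites its Keys value with KeyNumber, prints the acquired key's name from Names, then destroys the actor.
; The construction script applies the Material variable to the Key component, so each placed key can have its own look.
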(event EventBeginPlay
  (bind _asgame_mode_1 (Utilities|Casting|CastTogameMode1 (Game|GetGameMode)))
  (Variables|Default|SetgameMode _asgame_mode_1))

(event EventInteract
  (bind _output_get (Variables|/Game/a/gameMode1.gameMode1_C|SetKeys (Variables|Default|GetgameMode) (Variables|Default|GetKeyNumber)))
  (Development|PrintString (Utilities|String|Append "Key" (Utilities|Array|Get(acopy) (Variables|Default|GetNames) _output_get) "Acquired"))
  (Actor|DestroyActor))

(fn ConstructionScript
  (Rendering|Material|SetMaterial (Variables|Default|GetKey) 0 (Variables|Default|Getmaterial)))